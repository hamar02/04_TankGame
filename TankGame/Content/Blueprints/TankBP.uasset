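; Tank Blueprint that provides player-controlled camera orbit around the tank.
; The Azimuth axis yaws the AzimuthGimbal component and the Elavation axis pitches the SpringArm, keeping the two rotations on separate components.
; Both apply local rotation scaled by a shared Sensitivity and world delta seconds for frame-rate independence.
; The event graph and construction script hold no logic.
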(event EventBeginPlay)

(event Collision|EventActorBeginOverlap
  (params (OtherActor :type Actor%20Object%20Reference)))

(event EventTick
  (params (DeltaSeconds :type Float%20%28single-precision%29)))

(event Input|AxisEvents|InputAxisElavation
  (params (AxisValue :type Float%20%28single-precision%29))
  ;[1 1 1] Elavation
  (Transformation|AddLocalRotation (Variables|Default|GetSpringArm) (Math|Rotator|MakeRotator 0.0 (* AxisValue (Utilities|Time|GetWorldDeltaSeconds) (Variables|Default|GetSensitivity)) 0.0) false false))

(event Input|AxisEvents|InputAxisAzimuth
  (params (AxisValue :type Float%20%28single-precision%29))
  ;[1 1 1] Azimuth
  (Transformation|AddLocalRotation (Variables|Default|GetAzimuth%20Gimbal) (Math|Rotator|MakeRotator 0.0 0.0 (* AxisValue (Utilities|Time|GetWorldDeltaSeconds) (Variables|Default|GetSensitivity))) false false))

(fn ConstructionScript)